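; BP_CharacterBase is a base character Blueprint that exposes movement and combat state through interface getter functions.
; The getters return the aiming, crouching, jumping, reloading and sprinting flags, plus an aim offset obtained from GetAimOffset.
; It only passes state through: the event graph and construction script are empty, and nothing here sets those values or defines GetAimOffset.
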(fn `GetAiming_Interface`
  (returns (IsAiming :type Boolean))
  (return (`self.bIsAiming`)))

(fn `GetAimOffset_Interface`
  (returns (AimOffset :type "Rotator Structure"))
  (return (`self.GetAimOffset`)))

(fn `GetCrouching_Interface`
  (returns (IsCrouching :type Boolean))
  (return (`self.bIsCrouched`)))

(fn `GetJumping_Interface`
  (returns (IsJumping :type Boolean))
  (return (`self.bIsJumping`)))

(fn `GetReloading_Interface`
  (returns (Reloading :type Boolean))
  (return (`self.bIsReloading`)))

(fn `GetSprinting_Interface`
  (returns (IsSprinting :type Boolean))
  (return (`self.bIsSprinting`)))

(fn `UserConstructionScript`)